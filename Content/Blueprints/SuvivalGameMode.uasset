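; Survival game mode that runs the game-over, restart and quit flow and tracks the longest survival time.
; On BeginPlay it caches the GlobalTimer and Cabinet actors and the game instance, and shows the runtime UI.
; GameOver stops the timer and shows the failed panel with the survived day and hour.
; CheckScore compares total hours against the "bestScore" save slot, saves new records, and returns a Chinese result message.
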(event `self.ReceiveBeginPlay`
  (`|ExecutionSequence`
    (:`then_0`
      (bind _outactors (`GameplayStatics.GetAllActorsOfClass` "/Game/Blueprints/GlobalTImer.GlobalTimer_C"))
      (set `self.GlobalTimer` (`|GetArrayItem` _outactors))
      (`/Game/Blueprints/SurvivalGameInstance.ShowRuntimeUI` (cast `/Game/Blueprints/SurvivalGameInstance` (`GameplayStatics.GetGameInstance`) :!pure true)))
    (:`then_1`
      (bind _outactors_2 (`GameplayStatics.GetAllActorsOfClass` "/Game/Blueprints/Props/Cabinet.Cabinet_C"))
      (set `self.Cabinet` (`|GetArrayItem` _outactors_2)))
    (:`then_2`
      (set `self.GameInstance` (cast `/Game/Blueprints/SurvivalGameInstance` (`GameplayStatics.GetGameInstance`) :!pure true)))))

(event `GameOver`
  (bind _gameinstance (`self.GameInstance`))
  (bind _globaltimer (`self.GlobalTimer`))
  (bind _currentday (`/Game/Blueprints/GlobalTImer.CurrentDay` _globaltimer))
  (bind _currenthour (`/Game/Blueprints/GlobalTImer.CurrentHour` _globaltimer))
  (`/Game/Blueprints/GlobalTImer.StopTimer` (`self.GlobalTimer`))
  (`/Game/Blueprints/SurvivalGameInstance.HideAllPanels` _gameinstance)
  (`/Game/Blueprints/SurvivalGameInstance.ShowFailedPanel` _gameinstance)
  (bind _recordtext (`self.CheckScore` _currentday _currenthour))
  (`/Game/UI/UI_Failed.SetTexts` (`/Game/Blueprints/SurvivalGameInstance.FailedPanel` _gameinstance) _currentday _currenthour _recordtext))

(event `RestartGame`
  (`GameplayStatics.OpenLevel` "MainLevel"))

(event `QuitGame`
  (`KismetSystemLibrary.ExecuteConsoleCommand` "exit"))

(fn `CheckScore`
  (params (newDay :type Integer) (newHour :type Integer))
  (returns (RecordText :type String))
  (bind _returnvalue (`GameplayStatics.DoesSaveGameExist` "bestScore"))
  (if _returnvalue
    (bind _returnvalue_2 (`GameplayStatics.LoadGameFromSlot` "bestScore"))
    (bind _asbest_score (cast `/Game/Blueprints/BestScore` _returnvalue_2))
    (bind _bestday (`/Game/Blueprints/BestScore.BestDay` _asbest_score))
    (bind _besthour (`/Game/Blueprints/BestScore.BestHour` _asbest_score))
    (bind _returnvalue_3 (- (+ (* newDay 24) newHour) (+ (* _bestday 24) _besthour)))
    (if (> _returnvalue_3 0)
      _
      (elif (== _returnvalue_3 0)
        (return "加油，离打破记录之差一步之遥！")
        (else
          (return (`KismetStringLibrary.Concat_StrStr` "最长生存时间:" (`KismetStringLibrary.Conv_IntToString` _bestday) "天" (`KismetStringLibrary.Conv_IntToString` _besthour) "小时"))))))
  (bind _returnvalue_4 (`GameplayStatics.CreateSaveGameObject` "/Game/Blueprints/BestScore.BestScore_C"))
  (set `/Game/Blueprints/BestScore.BestDay` newDay _returnvalue_4)
  (set `/Game/Blueprints/BestScore.BestHour` newHour _returnvalue_4)
  (`GameplayStatics.SaveGameToSlot` _returnvalue_4 "bestScore")
  (return "恭喜，你创造了新纪录！"))

(fn `UserConstructionScript`)